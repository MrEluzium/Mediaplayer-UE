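; Overlay3D is an actor that presents a rotatable 3D mesh for the media player, with a scene capture restricted to its own components.
; Start resets the mesh orientation and enables a slow idle yaw spin on Tick until Stop.
; AddRotation applies 2D input as delta-time-scaled yaw and roll, pausing idle behavior.
; When idle with nonzero pitch, the PitchBackTime timeline eases roll and pitch back to zero.
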(event Custom|Start
  (Transformation|SetRelativeRotation (Variables|Default|GetStaticMesh) "0.000000,60.000000,0.000000" false false)
  (Variables|Default|SetbShown true))

(event Custom|Stop
  (Variables|Default|SetbShown false))

(event EventBeginPlay
  (Rendering|SceneCapture|ShowOnlyActorComponents (Variables|Default|GetSceneCaptureComponent2D) self false))

(event EventTick
  (params (DeltaSeconds :type Float%20%28single-precision%29))
  (bind _staticmesh (Variables|Default|GetStaticMesh))
  (bind _returnvalue (Transformation|GetWorldRotation _staticmesh))
  (Variables|Default|SetDT DeltaSeconds)
  (Utilities|FlowControl|Sequence
    (:then_0
      (if (and (Variables|Default|GetbShown) (Variables|Default|GetbIdleRotation))
        (Transformation|AddLocalRotation (Variables|Default|GetStaticMesh) (Math|Rotator|MakeRotator 0.0 0.0 (* (Variables|Default|GetDT) 1e+01)) false false)))
    (:then_1
      (if (and (!= (.pitch (.rotation (Transformation|GetRelativeTransform (Variables|Default|GetStaticMesh)))) 0.0) (Variables|Default|GetbIdleRotation))
        (bind _alpha (Timeline|PitchBackTime PlayFromStart)
          (:Update
            (Transformation|SetWorldRotation _staticmesh (Math|Rotator|MakeRotator (Math|Float|Lerp (.roll _returnvalue) 0.0 _alpha) (Math|Float|Lerp (.pitch _returnvalue) 0.0 _alpha) (.yaw _returnvalue)) false false)))
        (else
          (Timeline|PitchBackTime Stop))))))

(fn ConstructionScript)

(fn AddRotation
  (params (Rotation :type Vector%202D%20Structure))
  (bind _dt (Variables|Default|GetDT))
  (bind _returnvalue (* Rotation (Math|Vector2D|MakeVector2D _dt _dt)))
  (if (not (Class|KismetMathLibrary|IsZero2D Rotation))
    (Variables|Default|SetbIdleRotation false)
    (Transformation|AddWorldRotation (Variables|Default|GetStaticMesh) (Math|Rotator|MakeRotator (* (.y _returnvalue) -1.0) 0.0 (.x _returnvalue)) false false)
    (else
      (Variables|Default|SetbIdleRotation true))))